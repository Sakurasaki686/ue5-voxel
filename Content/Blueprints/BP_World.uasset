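; BP_World is the world Blueprint for a voxel game, setting up voxel materials and a stats UI when play begins.
; On BeginPlay it reads each row of the VoxelMaterials data table and constructs a VoxelMaterial object with that row's texture and ID, stored in Materials.
; The VoxelStats widget, bound to VoxelChunk, is created inside that loop, so one is added to the viewport per row found.
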(event EventBeginPlay
  ;[1 1 1] Load Materials
  (bind _outrownames (DataTable|GetDataTableRowNames "/Game/Blueprints/Data/VoxelMaterials.VoxelMaterials"))
  (for _array_element _outrownames
    (bind _returnvalue (Utilities|GetDataTableRow "/Game/Blueprints/Data/VoxelMaterials.VoxelMaterials" _array_element)
      (:then
        (bind _returnvalue_2 (Game|ConstructObjectfromClass self "/Script/Voxel.VoxelMaterial"))
        (Variables|/Script/Voxel.VoxelMaterial|SetTexture _returnvalue_2 (.texture _returnvalue))
        (Variables|/Script/Voxel.VoxelMaterial|SetId _returnvalue_2 (.id _returnvalue))
        (Utilities|Array|Add (Variables|Default|GetMaterials) _returnvalue_2)
        ;[1 1 1] Add Stats UI
        (bind _returnvalue_3 (UserInterface|CreateWidget "/Game/UI/VoxelStats.VoxelStats_C" (Game|GetPlayerController 0) (Variables|Default|GetVoxelChunk)))
        (UserInterface|Viewport|AddtoViewport _returnvalue_3 0)))))

(event Collision|EventActorBeginOverlap
  (params (OtherActor :type Actor%20Object%20Reference)))

(event EventTick
  (params (DeltaSeconds :type Float%20%28single-precision%29)))

(fn ConstructionScript)